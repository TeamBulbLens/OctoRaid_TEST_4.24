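; BP_Flag1 is a flag prop whose look is configured per instance through exposed variables.
; Its Construction Script creates a dynamic instance of M_Flag on element 1 of the flag mesh and pushes textures, colors, opacity, emissive, panning, tiling, fresnel and distance fade into it.
; The event graph is empty, so all setup happens at construction and any motion is left to the material.
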(fn `UserConstructionScript`
  (bind _mi_flag (`self.MI_Flag`))
  (bind _mi_flag_2 (`self.MI_Flag`))
  (bind _mi_flag_3 (`self.MI_Flag`))
  (bind _mi_flag_4 (`self.MI_Flag`))
  (bind _mi_flag_5 (`self.MI_Flag`))
  (bind _returnvalue (`PrimitiveComponent.CreateDynamicMaterialInstance` (`self.SM_Flag`) 1 "/Game/Neon_Materials/Materials/M_Flag/M_Flag.M_Flag" "M_Flag"))
  (set `self.MI_Flag` _returnvalue)
  (`|ExecutionSequence`
    (:`then_0`
      ;[1 1 1 1 28] Textures
      (`MaterialInstanceDynamic.SetTextureParameterValue` _mi_flag_3 "Opacity Mask" (`self.Opacity Mask`))
      (`MaterialInstanceDynamic.SetTextureParameterValue` _mi_flag_3 "Normal Map" (`self.Normal Map`))
      (`MaterialInstanceDynamic.SetTextureParameterValue` _mi_flag_3 "Panner Map" (`self.Panner Map`)))
    (:`then_1`
      ;[1 1 1 1 28] Opacity, Color, Emissive
      (`MaterialInstanceDynamic.SetScalarParameterValue` _mi_flag_4 "Opacity" (`self.Opacity`))
      (`MaterialInstanceDynamic.SetVectorParameterValue` _mi_flag_4 "Color 1" (`self.Color 1`))
      (`MaterialInstanceDynamic.SetVectorParameterValue` _mi_flag_4 "Color 2" (`self.Color 2`))
      (`MaterialInstanceDynamic.SetScalarParameterValue` _mi_flag_4 "Emissive" (`self.Emissive`)))
    (:`then_2`
      ;[1 1 1 1 28] Panners
      (`MaterialInstanceDynamic.SetScalarParameterValue` _mi_flag_5 "X Panner" (`self.X_Panner`))
      (`MaterialInstanceDynamic.SetScalarParameterValue` _mi_flag_5 "Y Panner" (`self.Y_Panner`)))
    (:`then_3`
      ;[1 1 1 1 28] UV Tiling
      (`MaterialInstanceDynamic.SetScalarParameterValue` _mi_flag_2 "U Tiling" (`self.U Tiling`))
      (`MaterialInstanceDynamic.SetScalarParameterValue` _mi_flag_2 "V Tiling" (`self.V Tiling`)))
    (:`then_4`
      ;[1 1 1 1 28] Fresnel
      (`MaterialInstanceDynamic.SetScalarParameterValue` _mi_flag "Fresnel" (`self.Fresnel`))
      (`MaterialInstanceDynamic.SetScalarParameterValue` _mi_flag "Rim Contrast" (`self.Rim Contrast`))
      (`MaterialInstanceDynamic.SetScalarParameterValue` _mi_flag "Distance Fade" (`self.Distance Fade`)))))