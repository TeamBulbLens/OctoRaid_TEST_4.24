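; Respawn area actor that supplies spawn transforms from random locations within its Box volume.
; GetRespawnPoint picks a random point in the box, line-traces downward against WorldStatic objects and returns the hit location, with yaw facing the world origin.
; A fallback returns the actor's center, but the branch condition is fixed to true, so it never runs and a missed trace goes unchecked.
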(fn `GetRespawnPoint`
  (returns (RespawnTransform :type "Transform Structure"))
  (locals (NewLocalVar_0 :type "Transform Structure"))
  (bind _returnvalue (`self.K2_GetActorLocation`))
  (bind (_returnvalue_roll _returnvalue_pitch _returnvalue_yaw) (`KismetMathLibrary.BreakRotator` (`KismetMathLibrary.FindLookAtRotation` _returnvalue (`KismetMathLibrary.MakeVector` 0.0))))
  (bind _returnvalue_2 (`KismetMathLibrary.RandomPointInBoundingBox` (`self.K2_GetActorLocation`) (`BoxComponent.GetScaledBoxExtent` (`self.Box`))))
  ;[1 1 1] box 볼륨 내 랜덤 위치를 리턴
  (bind _outhit (`KismetSystemLibrary.LineTraceSingleForObjects` _returnvalue_2 (+ _returnvalue_2 (* (`KismetMathLibrary.Vector_Down`) 1000.0)) (`|MakeArray` "ObjectTypeQuery1" :!type "EObjectTypeQuery Enum")))
  (if true
    (bind _returnvalue_3 (+ (`.Location` (`GameplayStatics.BreakHitResult` _outhit)) (0.0 0.0 0.0)))
    (bind (_returnvalue_roll_2 _returnvalue_pitch_2 _returnvalue_yaw_2) (`KismetMathLibrary.BreakRotator` (`KismetMathLibrary.FindLookAtRotation` _returnvalue_3 (`KismetMathLibrary.MakeVector` 0.0))))
    (return (`KismetMathLibrary.MakeTransform` _returnvalue_3 (`KismetMathLibrary.MakeRotator` 0.0 0.0 _returnvalue_yaw_2)))
    (else
      ;;[1 1 1] 랜덤 지점 가져오기가 실패할 경우 기본값으로 액터 가운데 지점 가져오기
      (return (`KismetMathLibrary.MakeTransform` _returnvalue (`KismetMathLibrary.MakeRotator` 0.0 0.0 _returnvalue_yaw))))))

(fn `UserConstructionScript`)