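; BP_ItemSpawner is a hunter item spawner that spawns the ItemToLoad class at its own transform, on the authority only.
; Tick calls ServerSpawnItem every frame and again whenever the RespawnDelay Delay completes, so the delay does not throttle it.
; Respawn alternates on IsSpawn between spawning and re-arming, without checking for an existing item.
; The node setting Item1's child actor class is unconnected.
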(event `self.ReceiveBeginPlay`)

(event `self.ReceiveTick`
  (params (DeltaSeconds :type "Float (single-precision)"))
  (`self.ServerspawnItem` :!label _label)
  (`KismetSystemLibrary.Delay` (`self.RespawnDelay`))
  (goto _label))

(event `ServerSpawnItem`
  (`/Engine/EditorBlueprintResources/ActorMacros.Switch Has Authority`
    (:`Authority`
      (`self.Respawn`))))

(fn `Respawn`
  (if (`self.IsSpawn?`)
    (`|SpawnActorFromClass` (`self.ItemToLoad`) (`self.GetTransform` (`ActorComponent.GetOwner` (`self.Item_1`))) "Undefined" "OverrideRootScale" null null)
    (set `self.IsSpawn?` false)
    (else
      (set `self.IsSpawn?` true))))

(fn `UserConstructionScript`)