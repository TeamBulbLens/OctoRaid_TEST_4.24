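; BP_Dome is a configurable neon dome actor whose look is set through exposed variables, with no active runtime logic.
; The Construction Script creates a dynamic instance of M_Dome on the SMDome mesh.
; It then pushes the variables into that instance in grouped steps: mask and noise textures, two colors, panning, UV tiling, Fresnel rim with distance fade, and noise distortion.
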(fn `UserConstructionScript`
  (bind _mi_dome (`self.MI_Dome`))
  (bind _mi_dome_2 (`self.MI_Dome`))
  (bind _mi_dome_3 (`self.MI_Dome`))
  (bind _mi_dome_4 (`self.MI_Dome`))
  (bind _mi_dome_5 (`self.MI_Dome`))
  (bind _mi_dome_6 (`self.MI_Dome`))
  (bind _returnvalue (`PrimitiveComponent.CreateDynamicMaterialInstance` (`self.SM_Dome`) 0 "/Game/Neon_Materials/Materials/M_Dome/M_Dome.M_Dome" "M_Dome"))
  (set `self.MI_Dome` _returnvalue)
  (`|ExecutionSequence`
    (:`then_0`
      ;[1 1 1 1 28] Textures
      (`MaterialInstanceDynamic.SetTextureParameterValue` _mi_dome_4 "Opacity Mask" (`self.Opacity Mask`))
      (`MaterialInstanceDynamic.SetTextureParameterValue` _mi_dome_4 "Noise Map" (`self.Noise Map`)))
    (:`then_1`
      ;[1 1 1 1 28] Opacity, Color, Emissive
      (`MaterialInstanceDynamic.SetVectorParameterValue` _mi_dome_5 "Color 1" (`self.Color 1`))
      (`MaterialInstanceDynamic.SetVectorParameterValue` _mi_dome_5 "Color 2" (`self.Color 2`)))
    (:`then_2`
      ;[1 1 1 1 28] Panners
      (`MaterialInstanceDynamic.SetScalarParameterValue` _mi_dome_6 "X Panner" (`self.X_Panner`))
      (`MaterialInstanceDynamic.SetScalarParameterValue` _mi_dome_6 "Y Panner" (`self.Y_Panner`)))
    (:`then_3`
      ;[1 1 1 1 28] UV Tiling
      (`MaterialInstanceDynamic.SetScalarParameterValue` _mi_dome_3 "U Tiling" (`self.U Tiling`))
      (`MaterialInstanceDynamic.SetScalarParameterValue` _mi_dome_3 "V Tiling" (`self.V Tiling`)))
    (:`then_4`
      ;[1 1 1 1 28] Fresnel
      (`MaterialInstanceDynamic.SetScalarParameterValue` _mi_dome "Fresnel" (`self.Fresnel`))
      (`MaterialInstanceDynamic.SetScalarParameterValue` _mi_dome "Rim Contrast" (`self.Rim Contrast`))
      (`MaterialInstanceDynamic.SetScalarParameterValue` _mi_dome "Distance Fade" (`self.Distance Fade`)))
    (:`then_5`
      ;[1 1 1] Distortion
      (`MaterialInstanceDynamic.SetScalarParameterValue` _mi_dome_2 "X Panner Noise" (`self.X Panner Noise`))
      (`MaterialInstanceDynamic.SetScalarParameterValue` _mi_dome_2 "Y Panner Noise" (`self.Y Panner Noise`))
      (`MaterialInstanceDynamic.SetScalarParameterValue` _mi_dome_2 "Noise" (`self.Noise`)))))