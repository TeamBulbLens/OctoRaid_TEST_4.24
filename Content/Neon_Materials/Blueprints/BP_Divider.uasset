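; BP_Divider is a configurable divider prop with a band mesh and optional start and end poles, from the Neon_Materials content.
; The Construction Script creates a dynamic instance of M_Band and feeds it textures, opacity, color, emissive, panning and tiling from Blueprint variables.
; VTiling drives the "U Normal Tiling" parameter, despite its name.
; Two toggles set each pole's visibility and collision together, and the Event Graph holds no active logic.
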(fn `UserConstructionScript`
  (bind _mi_divider (`self.MI_Divider`))
  (bind _sm_divider_pole__end_pole_ (`self.SM_Divider_Pole (End Pole)`))
  (bind _sm_divider_pole__start_pole_ (`self.SM_Divider_Pole (Start Pole)`))
  (bind _mi_divider_2 (`self.MI_Divider`))
  (bind _mi_divider_3 (`self.MI_Divider`))
  (bind _mi_divider_4 (`self.MI_Divider`))
  (bind _returnvalue (`PrimitiveComponent.CreateDynamicMaterialInstance` (`self.SM_Band`) 0 "/Game/Neon_Materials/Materials/M_Band/M_Band.M_Band" "M_Band"))
  (set `self.MI_Divider` _returnvalue)
  (`|ExecutionSequence`
    (:`then_0`
      ;[1 1 1 1 28] Textures
      (`MaterialInstanceDynamic.SetTextureParameterValue` _mi_divider_2 "Opacity Mask" (`self.Opacity Mask`))
      (`MaterialInstanceDynamic.SetTextureParameterValue` _mi_divider_2 "Normal Map" (`self.Normal Map`))
      (`MaterialInstanceDynamic.SetTextureParameterValue` _mi_divider_2 "Panner Map" (`self.Panner Map`)))
    (:`then_1`
      ;[1 1 1 1 28] Opacity, Color, Emissive
      (`MaterialInstanceDynamic.SetScalarParameterValue` _mi_divider_3 "Opacity" (`self.Opacity`))
      (`MaterialInstanceDynamic.SetVectorParameterValue` _mi_divider_3 "Color" (`self.Color`))
      (`MaterialInstanceDynamic.SetScalarParameterValue` _mi_divider_3 "Emissive" (`self.Emissive`)))
    (:`then_2`
      ;[1 1 1 1 28] Panners
      (`MaterialInstanceDynamic.SetScalarParameterValue` _mi_divider_4 "X Panner" (`self.X_Panner`))
      (`MaterialInstanceDynamic.SetScalarParameterValue` _mi_divider_4 "Y Panner" (`self.Y_Panner`))
      (`MaterialInstanceDynamic.SetScalarParameterValue` _mi_divider_4 "X Normal Panner" (`self.X Normal Panner`))
      (`MaterialInstanceDynamic.SetScalarParameterValue` _mi_divider_4 "Y Normal Panner" (`self.Y Normal Panner`)))
    (:`then_3`
      ;[1 1 1 1 28] UV Tiling
      (`MaterialInstanceDynamic.SetScalarParameterValue` _mi_divider "U Tiling" (`self.U Tiling`))
      (`MaterialInstanceDynamic.SetScalarParameterValue` _mi_divider "U Normal Tiling" (`self.V Tiling`)))
    (:`then_4`
      ;[1 1 1 1 28] Mesh
      (if (`self.Use End Pole`)
        (`SceneComponent.SetVisibility` _sm_divider_pole__end_pole_ true true)
        (`PrimitiveComponent.SetCollisionEnabled` _sm_divider_pole__end_pole_ "QueryAndPhysics")
        (else
          (`SceneComponent.SetVisibility` _sm_divider_pole__end_pole_ false true)
          (`PrimitiveComponent.SetCollisionEnabled` _sm_divider_pole__end_pole_ "NoCollision")))
      (if (`self.Use Start Pole`)
        (`SceneComponent.SetVisibility` _sm_divider_pole__start_pole_ true true)
        (`PrimitiveComponent.SetCollisionEnabled` _sm_divider_pole__start_pole_ "QueryAndPhysics")
        (else
          (`SceneComponent.SetVisibility` _sm_divider_pole__start_pole_ false true)
          (`PrimitiveComponent.SetCollisionEnabled` _sm_divider_pole__start_pole_ "NoCollision"))))))