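; BP_Projectile_SN is a bullet projectile actor with a limited lifespan that damages what it overlaps.
; On BeginPlay it takes its damage value from BP_MainGM, the game mode.
; On collision overlap it applies damage credited to player controller 0, spawns an impact emitter and sound, then destroys itself.
; The gun-sound server-to-multicast chain is an uncalled stub with an empty final event, and BulletMove is empty.
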(event `self.ReceiveBeginPlay`
  ;[1 1 1] Bullet
  (`self.SetLifeSpan` (`self.BulletLife`))
  (bind _asbp_main_gm (cast `/Game/Blueprints/System/Main/BP_MainGM` (`GameplayStatics.GetGameMode`)))
  (set `self.BulletDamage` (`/Game/Blueprints/System/Main/BP_MainGM.BulletDamage` _asbp_main_gm)))

(event `BulletMove`
  ;[1 1 1] Bullet
)

(event `self.BulletCollision.OnComponentBeginOverlap`
  (params (OverlappedComponent :type "PrimitiveComponent Object Reference") (OtherActor :type "Actor Object Reference") (OtherComp :type "PrimitiveComponent Object Reference") (OtherBodyIndex :type Integer) (bFromSweep :type Boolean) (SweepResult :type "HitResult Structure (by ref)"))
  (bind _returnvalue (`SceneComponent.K2_GetComponentLocation` (`self.BulletCollision`)))
  ;[1 1 1] Overlap
  (`GameplayStatics.ApplyDamage` OtherActor (`self.BulletDamage`) (`GameplayStatics.GetPlayerController` 0) self)
  (`GameplayStatics.SpawnEmitterAtLocation` "/Game/LJM/P_OR/P_Bullet_final_01.P_Bullet_final_01" _returnvalue (struct) (5.0 5.0 5.0))
  (`GameplayStatics.SpawnSoundAtLocation` "/Game/Ultimate_SFX_Bundle/Warfare_SFX_Bundle/Bullet_Impacts_Flybys_Pro/Cues/Snow/Snow_6_Cue.Snow_6_Cue" _returnvalue (struct) 5.0 1.0 0.0 null null)
  (`self.K2_DestroyActor`))

(event `PlayGunSound`
  (`self.ServerGunSound` (`SceneComponent.K2_GetComponentLocation` (`self.BulletCollision`))))

(event `ServerGunSound`
  (params (SoundLocation :type "Vector Structure"))
  (`self.MulticastGunSound` SoundLocation))

(event `MulticastGunSound`
  (params (SoundLocation :type "Vector Structure")))

(fn `UserConstructionScript`)